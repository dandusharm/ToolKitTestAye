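; Mind control status effect that temporarily turns the affected unit to the caster's side under AI control.
; Activation saves the unit's allied factions and AI flag, copies the active unit's factions, enables AI control and queues a MindControl action, which turn start also queues.
; Animating the Mind Control action plays a possession particle and sound, then ends after a short delay.
; Turn end restores the saved values and disables the effect.
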(event EventAnimateAction
  (params (Action :type F%20Action%20Structure))
  (bind _unit (CallFunction|GetUnit Action))
  (bind _returnvalue (Transformation|GetActorLocation _unit))
  (switch name (CallFunction|GetActionName Action)
    (:Default
      (|CallParentFunction Action))
    (:MindControl
      (Effects|SpawnEmitteratLocation "/Game/AdvancedTurnBasedTileToolkit/Maps/Advanced/Abilities/PS_Posseser_Attach.PS_Posseser_Attach" _returnvalue)
      (Audio|PlaySoundatLocation "/Game/AdvancedTurnBasedTileToolkit/Maps/Advanced/Abilities/A_MindControl.A_MindControl" _returnvalue "0, 0, 0" 1.0 1.0 0.0 0 0 0)
      (Utilities|FlowControl|Delay 1.0)
      (Utilities|EndAction))))

(event EventActivate
  (params (Target%20Unit :type BP%20Unit%20Object%20Reference))
  (bind _owningunit (Variables|Default|GetOwningUnit))
  (|CallParentFunction Target%20Unit)
  (Variables|Default|SetOldAlliedFactions (Variables|/Game/AdvancedTurnBasedTileToolkit/Core/Units/BP_Unit.BP_Unit_C|GetAlliedFactions _owningunit))
  (Variables|Default|SetbOldAIControlled (Variables|/Game/AdvancedTurnBasedTileToolkit/Core/Units/BP_Unit.BP_Unit_C|GetbAIControlled _owningunit))
  (bind _turnmanager (Class|BPISingletons|FindTurnManagerinState(Message) (Game|GetGameState)))
  (Variables|/Game/AdvancedTurnBasedTileToolkit/Core/Units/BP_Unit.BP_Unit_C|SetAlliedFactions (Variables|Default|GetOwningUnit) (Variables|/Game/AdvancedTurnBasedTileToolkit/Core/Units/BP_Unit.BP_Unit_C|GetAlliedFactions (Variables|/Game/AdvancedTurnBasedTileToolkit/Core/BP_TurnManager.BP_TurnManager_C|GetActiveUnit _turnmanager)))
  (Variables|/Game/AdvancedTurnBasedTileToolkit/Core/Units/BP_Unit.BP_Unit_C|SetbAIControlled (Variables|Default|GetOwningUnit) true)
  (Utilities|QueueActionSingles :Executing%20Object self :Action%20Name "MindControl" :Unit (Variables|Default|GetOwningUnit)))

(event EventRunonTurnStart
  (Utilities|QueueActionSingles :Executing%20Object self :Action%20Name "MindControl" :Unit (Variables|Default|GetOwningUnit)))

(event EventRunonTurnEnd
  (Variables|/Game/AdvancedTurnBasedTileToolkit/Core/Units/BP_Unit.BP_Unit_C|SetAlliedFactions (Variables|Default|GetOwningUnit) (Variables|Default|GetOldAlliedFactions))
  (Variables|/Game/AdvancedTurnBasedTileToolkit/Core/Units/BP_Unit.BP_Unit_C|SetbAIControlled (Variables|Default|GetOwningUnit) (Variables|Default|GetbOldAIControlled))
  (CallFunction|Disable))

(fn ConstructionScript
  (|CallParentFunction))